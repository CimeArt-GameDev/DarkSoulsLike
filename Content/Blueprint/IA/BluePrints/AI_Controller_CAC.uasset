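; AI controller for the CAC enemy that starts the BT_CAC behavior tree on BeginPlay.
; When AI perception updates on a ThirdPersonCharacter, it writes whether the stimulus was successfully sensed into the "Seen" blackboard key for the tree to use.
; Leftover unconnected nodes include a debug print and a PlayerActor blackboard write that never run.
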(event `self.ReceiveBeginPlay`
  (`self.RunBehaviorTree` "/Game/Blueprint/IA/BehaviorTree/BT_CAC.BT_CAC"))

(event `self.AIPerception.OnTargetPerceptionUpdated`
  (params (Actor :type "Actor Object Reference") (Stimulus :type "AIStimulus Structure"))
  (cast `/Game/Blueprint/ThirdPersonCharacter` Actor)
  (`BlackboardComponent.SetValueAsBool` (`AIBlueprintHelperLibrary.GetBlackboard` null) "Seen" (`.bSuccessfullySensed` (break `AIStimulus` Stimulus))))

(fn `UserConstructionScript`)