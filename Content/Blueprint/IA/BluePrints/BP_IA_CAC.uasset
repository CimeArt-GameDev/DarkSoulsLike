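; BP_IA_CAC is an AI-controlled character, likely a melee (CAC) enemy, with life, movement speed and an attack state.
; TakeDamage subtracts Life, then blocks further damage for one second.
; BeginPlay applies the walk speed and creates a life bar widget referencing itself, which Tick yaws toward the BP_Player_Thibault pawn.
; StartAttack only sets the Attacking flag; no death or attack logic lives here.
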(event `Take Damage`
  (params (Damage :type "Float (double-precision)"))
  (if (`self.canTakeDmg?`)
    (set `self.Life` (- (`self.Life`) Damage))
    (set `self.canTakeDmg?` false)
    (`KismetSystemLibrary.Delay` 1.0)
    (set `self.canTakeDmg?` true)))

(event `self.ReceiveTick`
  (params (DeltaSeconds :type "Float (single-precision)"))
  (bind _widget (`self.Widget`))
  (bind _asbp_player_thibault (cast `/Game/ThirdPersonBP/Blueprints/BP_Player_Thibault` (`GameplayStatics.GetPlayerPawn` 0)))
  (bind (_returnvalue_roll _returnvalue_pitch _returnvalue_yaw) (`KismetMathLibrary.BreakRotator` (`KismetMathLibrary.FindLookAtRotation` (`SceneComponent.K2_GetComponentLocation` _widget) (`self.K2_GetActorLocation` _asbp_player_thibault))))
  (`SceneComponent.K2_SetRelativeRotation` _widget (`KismetMathLibrary.MakeRotator` 0.0 0.0 (- _returnvalue_yaw 90.0)) false false))

(event `self.ReceiveBeginPlay`
  (set `CharacterMovementComponent.MaxWalkSpeed` (`self.Movement speed`) (`self.CharacterMovement`))
  (bind _returnvalue (`|CreateWidget` "/Game/Blueprint/Widget/WG_IALifeBar.WG_IALifeBar_C" null self))
  (`WidgetComponent.SetWidget` (`self.Widget`) _returnvalue))

(event `StartAttack`
  (if (not (`self.Attacking`))
    (set `self.Attacking` true)))

(fn `UserConstructionScript`)