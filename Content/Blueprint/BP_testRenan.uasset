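; BP_testRenan is a test Blueprint for the characteristics menu and the stats data behind it.
; It shows the mouse cursor on BeginPlay, and E toggles a WG_CaracMenu widget that receives Stats on creation.
; F adds 100 to the Attribut of every entry in the Stats Caractéristique array.
; Tick prints the first entry's Attribut to screen as a live debug readout.
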(event `self.ReceiveBeginPlay`
  (set `PlayerController.bShowMouseCursor` true (`GameplayStatics.GetPlayerController` 0)))

(event `Key|E`
  (params (Key :type "Key Structure"))
  (:`Pressed`
    (`/Engine/EditorBlueprintResources/StandardMacros.FlipFlop`
      (:`A`
        (`/Engine/EditorBlueprintResources/StandardMacros.IsValid` (`self.WG_Carac`)
          (:`Is Not Valid`
            (bind _returnvalue (`|CreateWidget` "/Game/Blueprint/Widget/WG_CaracMenu.WG_CaracMenu_C" null (`self.Stats`)))
            (bind _output_get (set `self.WG_Carac` _returnvalue))
            (`UserWidget.AddToViewport` _output_get 0))))
      (:`B`
        (`Widget.RemoveFromParent` (`self.WG_Carac`))
        (set `self.WG_Carac` null)))))

(event `Key|F` :paused true
  (params (Key :type "Key Structure"))
  (bind (_player_name `_caractéristique`) (break `/Game/Blueprint/Struc/Struc_Carac` (`self.Stats`)))
  (:`Pressed`
    (for (_ _array_index) (`.Caractéristique_30_0A1D56C246203CD229E1149A04C9A083` (break `/Game/Blueprint/Struc/Struc_Carac` (`self.Stats`)))
      (bind (_output_name _output_attribut _output_preview) (break `/Game/Blueprint/Struc/Struc_CaracPreview` (`|GetArrayItem` `_caractéristique` _array_index)))
      (`KismetArrayLibrary.Array_Set` `_caractéristique` _array_index (make `/Game/Blueprint/Struc/Struc_CaracPreview` _output_name (+ _output_attribut 100) _output_preview)))))

(event `self.ReceiveTick`
  (params (DeltaSeconds :type "Float (single-precision)"))
  (bind (_stats_player_name `_stats_caractéristique`) (break `/Game/Blueprint/Struc/Struc_Carac` (`self.Stats`)))
  (bind (_output_name _output_attribut) (break `/Game/Blueprint/Struc/Struc_CaracPreview` (`|GetArrayItem` `_stats_caractéristique`)))
  (`KismetSystemLibrary.PrintString` (`KismetStringLibrary.Conv_IntToString` _output_attribut) true true (struct :`G` 0.66 :`B` 1.0 :`A` 1.0) 0.001))

(fn `UserConstructionScript`)